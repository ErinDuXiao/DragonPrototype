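; Test actor that travels along the looping spline of a BP_DragonRoute found in the level at BeginPlay.
; Each Tick grows a travel distance by Speed times delta time and asks the route for the location at that distance.
; The actor eases toward it with a fixed-alpha lerp, so the smoothing is frame-rate dependent.
; MaxSplinePoint is stored but never read, and a debug print is disconnected.
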(event EventBeginPlay
  (bind _outactors (Actor|GetAllActorsOfClass "/Game/BP/BP_DragonRoute.BP_DragonRoute_C"))
  (bind _output_get (Variables|Default|SetSpline (Utilities|Array|Get(acopy) _outactors)))
  (bind _returnvalue (Default|GetSplinePointNumber _output_get))
  (Variables|Default|SetMaxSplinePoint (Math|Conversions|ToFloat(Integer) _returnvalue)))

(event Collision|EventActorBeginOverlap
  (params (OtherActor :type Actor%20Object%20Reference)))

(event EventTick
  (params (DeltaSeconds :type Float%20%28single-precision%29))
  (bind _output_get (Variables|Default|SetMoveDist (+ (* DeltaSeconds (Variables|Default|GetSpeed)) (Variables|Default|GetMoveDist))))
  (bind _returnvalue (Default|GetCurrentLocation (Variables|Default|GetSpline) true _output_get))
  (Transformation|SetActorLocation (Math|Vector|Lerp(Vector) (Transformation|GetActorLocation) _returnvalue 0.01) false false))

(fn ConstructionScript)