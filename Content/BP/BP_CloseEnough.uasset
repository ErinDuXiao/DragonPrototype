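; BP_CloseEnough is a behavior tree decorator for the dragon AI that gates on the controlled pawn's distance to its follow target.
; It casts the owner to BP_DragonAIController, then measures from that pawn to the blackboard's TargetToFollow actor.
; Despite the name, the condition passes when that distance is at least AdaptableDistance, meaning the dragon is not yet close.
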(fn PerformConditionCheck
  (params (OwnerActor :type Actor%20Object%20Reference))
  (bind _asbp_dragon_aicontroller (Utilities|Casting|CastToBP_DragonAIController OwnerActor))
  (Variables|Default|SetAIConRef _asbp_dragon_aicontroller)
  (return (>= (Math|Vector|VectorLength (- (Transformation|GetActorLocation (AI|BehaviorTree|GetBlackboardValueasActor (Variables|Default|GetTargetToFollow))) (Transformation|GetActorLocation (Pawn|GetControlledPawn (Variables|Default|GetAIConRef))))) (Variables|Default|GetAdaptableDistance))))