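; Dragon actor that patrols along the first BP_DragonRoute in the level until it switches to chasing the player, setting head and body part classes for its parent class.
; Each tick it sphere-traces around the head and line-traces to hits for visibility.
; A visible hit, or route arrival checked during that loop, permanently latches HasFoundPlayer.
; TargetLocation follows the looping spline point until then, and the player pawn afterwards.
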(event Custom|FindTarget2
  (bind _head (Variables|Default|GetHead))
  (bind _splinepastlength (Variables|Default|GetSplinePastLength))
  (bind _dragonroutespline (Variables|Default|GetDragonRouteSpline))
  (bind _returnvalue (Transformation|GetActorLocation _head))
  (bind _returnvalue_2 (* _splinepastlength 3e+02))
  (if (Variables|Default|GetHasFoundPlayer)
    (Variables|Default|SetTargetLocation (Transformation|GetActorLocation (Game|Player|GetPlayerPawn 0)) :!label _label)
    (else
      (bind _outhits (Collision|MultiSphereTraceForObjects _returnvalue (+ _returnvalue "0, 0,15.000000") 1e+03 (Variables|Default|GetDesiredObjectType) false 0 "None" true "(R=1.000000,G=0.000000,B=0.000000,A=1.000000)" "(R=0.000000,G=1.000000,B=0.000000,A=1.000000)" 0.0))
      (bind _array_element (Utilities|Array|ForEachLoopwithBreak _outhits)
        (:LoopBody
          (bind _outhit (Collision|LineTraceByChannel _returnvalue (Transformation|GetActorLocation (.HitActor (Collision|BreakHitResult _array_element))) "TraceTypeQuery2" false 0 "None"))
          (if (== (Utilities|GetClass (.HitActor (Collision|BreakHitResult _outhit))) (Utilities|GetClass (.HitActor (Collision|BreakHitResult _array_element))))
            (Variables|Default|SetHasFoundPlayer true :!label _label_2)
            (goto _label)
            (else
              (bind _returnvalue_3 (Default|IsArrived _dragonroutespline _returnvalue_2))
              (if _returnvalue_3
                (goto _label_2)
                (else
                  _)))))
        (:Completed
          _))
      (bind _returnvalue_4 (Default|GetCurrentLocation _dragonroutespline true _returnvalue_2))
      (Variables|Default|SetTargetLocation _returnvalue_4))))

(event EventBeginPlay
  (|CallParentFunction)
  (bind _outactors (Actor|GetAllActorsOfClass "/Game/BP/BP_DragonRoute.BP_DragonRoute_C"))
  (Variables|Default|SetDragonRouteSpline (Utilities|Array|Get(acopy) _outactors)))

(event Collision|EventActorBeginOverlap
  (params (OtherActor :type Actor%20Object%20Reference))
  (|CallParentFunction OtherActor))

(event EventTick
  (params (DeltaSeconds :type Float%20%28single-precision%29))
  (|CallParentFunction DeltaSeconds)
  (CallFunction|FindTarget2))

(fn ConstructionScript
  (Variables|Default|SetHeadPartClass "/Game/BP/BP_DragonHeadTMP.BP_DragonHeadTMP_C")
  (Variables|Default|SetBodyPartClass "/Game/BP/BP_DragonBodyTMP.BP_DragonBodyTMP_C"))