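; Spline-based route actor, named for a dragon, that answers position and progress queries along its path.
; GetCurrentLocation scales Length by 100 into a world-space spline location; with Loop set, it applies a modulo by spline length, before scaling, once within 400 units of the end.
; IsArrived compares unscaled Length to spline length, and other helpers return that length, the point count and point locations.
; The event graph and construction script are empty.
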(event EventBeginPlay)

(event Collision|EventActorBeginOverlap
  (params (OtherActor :type Actor%20Object%20Reference)))

(event EventTick
  (params (DeltaSeconds :type Float%20%28single-precision%29)))

(fn ConstructionScript)

(fn GetCurrentLocation
  (params (Loop :type Boolean) (Length :type Float%20%28single-precision%29))
  (bind _spline (Variables|Default|GetSpline))
  (bind _returnvalue (Spline|GetSplineLength _spline))
  (if Loop
    (if (>= (+ (* Length 1e+02) 4e+02) _returnvalue)
      (Variables|Default|SetLocalLength (* (Math|Float|%(Float) Length _returnvalue) 1e+02))
      (else
        ;[1 1 1] local?
        (Variables|Default|SetLocalLength (* Length 1e+02) :!label _label)))
    (else
      (goto _label)))
  (return (Spline|GetLocationatDistanceAlongSpline (Variables|Default|GetSpline) (Variables|Default|GetLocalLength) "World")))

(fn GetSplineLength
  (return (Spline|GetSplineLength (Variables|Default|GetSpline))))

(fn IsArrived
  (params (length :type Float%20%28single-precision%29))
  (return (>= length (Spline|GetSplineLength (Variables|Default|GetSpline)))))

(fn GetLocationat
  (params (PointIndex :type Integer))
  (return (Spline|GetLocationatSplinePoint (Variables|Default|GetSpline) PointIndex "World")))

(fn GetSplinePointNumber
  (return (Spline|GetNumberOfSplinePoints (Variables|Default|GetSpline))))