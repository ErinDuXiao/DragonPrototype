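; BP_DragonHeadTMP is an end-of-game trigger actor, apparently standing in for the dragon's head.
; On BeginPlay it caches the first BP_Dragon found in the level.
; When the player pawn overlaps it, it creates and displays the WG_EndScreen widget and sets IsGameFinished on that dragon.
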(event EventBeginPlay
  (bind _outactors (Actor|GetAllActorsOfClass "/Game/BP/BP_Dragon.BP_Dragon_C"))
  (Variables|Default|SetDragonActorRef (Utilities|Array|Get(acopy) _outactors)))

(event Collision|EventActorBeginOverlap
  (params (OtherActor :type Actor%20Object%20Reference))
  (if (== OtherActor (Game|Player|GetPlayerPawn 0))
    (bind _returnvalue (UserInterface|CreateWidget "/Game/BP/WG_EndScreen.WG_EndScreen_C" (Game|GetPlayerController 0)))
    (UserInterface|Viewport|AddtoViewport _returnvalue 0)
    (Variables|/Script/DragonProto.DragonBase|SetIsGameFinished (Variables|Default|GetDragonActorRef) true)))

(event EventTick
  (params (DeltaSeconds :type Float%20%28single-precision%29)))

(fn ConstructionScript)