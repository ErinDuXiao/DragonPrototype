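; Dragon variant Blueprint that selects which head and body part classes the dragon uses.
; The construction script assigns the TMP head and body classes, while BeginPlay, overlap and Tick only forward to the parent.
; An unconnected debug snippet would print the turn direction from the head toward the player's pawn, but it never runs.
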(event EventBeginPlay
  (|CallParentFunction))

(event Collision|EventActorBeginOverlap
  (params (OtherActor :type Actor%20Object%20Reference))
  (|CallParentFunction OtherActor))

(event EventTick
  (params (DeltaSeconds :type Float%20%28single-precision%29))
  (|CallParentFunction DeltaSeconds))

(fn ConstructionScript
  (Variables|Default|SetHeadPartClass "/Game/BP/BP_DragonHeadTMP.BP_DragonHeadTMP_C")
  (Variables|Default|SetBodyPartClass "/Game/BP/BP_DragonBodyTMP.BP_DragonBodyTMP_C"))